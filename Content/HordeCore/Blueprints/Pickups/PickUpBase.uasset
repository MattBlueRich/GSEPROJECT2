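; Base pickup actor that grants a stats effect component to the first-person player character on touch.
; Its construction script reads the mesh and colour from the effect class defaults and feeds them, with scale and position offset, into Niagara for display.
; Overlapping the sphere passes the effect class to the character through AddPickUpComponentMessage, then destroys the pickup.
; The effect class thus drives both the pickup's look and what it grants.
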(event `self.Sphere.OnComponentBeginOverlap`
  (params (OverlappedComponent :type "PrimitiveComponent Object Reference") (OtherActor :type "Actor Object Reference") (OtherComp :type "PrimitiveComponent Object Reference") (OtherBodyIndex :type Integer) (bFromSweep :type Boolean) (SweepResult :type "HitResult Structure (by ref)"))
  (cast `/Game/FirstPerson/Blueprints/BP_FirstPersonCharacter` OtherActor)
  (message `/Game/HordeCore/Blueprints/Pickups/I_Pickup.AddPickUpComponent` OtherActor (`self.PickUpStatsEffectComponent`))
  (`self.K2_DestroyActor`))

(fn `InitialiseFromSpawn`
  (bind _pickupstatseffectcomponent (`self.PickUpStatsEffectComponent`))
  (bind (_pickupmesh _colour) (defaults `Object` _pickupstatseffectcomponent))
  (if (`KismetSystemLibrary.IsValidClass` _pickupstatseffectcomponent)
    (set `self.IconMesh` _pickupmesh)
    (set `self.Color` _colour)
    (`NiagaraComponent.SetVariableLinearColor` (`self.Niagara`) "Color01" (`self.Color`))
    (`NiagaraComponent.SetVariableStaticMesh` (`self.Niagara`) "mesh" (`self.IconMesh`))
    (`NiagaraComponent.SetVariableVec3` (`self.Niagara`) "MeshScale" (`self.MeshScale`))
    (`NiagaraComponent.SetVariablePosition` (`self.Niagara`) "Position" (`self.MeshPositionOffset`))))

(fn `UserConstructionScript`
  (`self.InitialiseFromSpawn`))