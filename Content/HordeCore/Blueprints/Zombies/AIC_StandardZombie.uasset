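; AI controller for standard horde zombies that runs the BT_StandardZombie behavior tree when it possesses a pawn.
; On possession it stores the zombie's animation blueprint in the blackboard, supporting both BP_StandardZombie and BP_Zombie pawns.
; Every tick, if the blackboard has no valid target, it assigns the first actor tagged Player.
; Helper functions write the target and line-of-sight keys to the blackboard.
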(event `self.ReceivePossess`
  (params (PossessedPawn :type "Pawn Object Reference"))
  (`self.RunBehaviorTree` "/Game/HordeCore/Blueprints/Zombies/BT_StandardZombie.BT_StandardZombie")
  (bind _asbp_standard_zombie (cast `/Game/HordeCore/Blueprints/Zombies/BP_StandardZombie` PossessedPawn)
    (:`then`
      (bind _asabp_standard_zombie (cast `/Game/HordeCore/Blueprints/Zombies/ABP_StandardZombie` (`SkeletalMeshComponent.GetAnimInstance` (`Character.Mesh` _asbp_standard_zombie))))
      (`BlackboardComponent.SetValueAsObject` (`self.Blackboard`) (`KismetStringLibrary.Conv_StringToName` "AnimBP") _asabp_standard_zombie))
    (:`CastFailed`
      (bind _asbp_zombie (cast `/Game/HordeCore/Blueprints/Zombies/BP_Zombie` PossessedPawn))
      (bind _asabp_zombie (cast `/Game/HordeCore/Blueprints/Zombies/ABP_Zombie` (`SkeletalMeshComponent.GetAnimInstance` (`/Game/HordeCore/Blueprints/Zombies/BP_Zombie.Mesh` _asbp_zombie))))
      (`BlackboardComponent.SetValueAsObject` (`self.Blackboard`) (`KismetStringLibrary.Conv_StringToName` "AnimBP") _asabp_zombie))))

(event `self.ReceiveTick`
  (params (DeltaSeconds :type "Float (single-precision)"))
  (`/Engine/EditorBlueprintResources/StandardMacros.IsValid` (`BlackboardComponent.GetValueAsObject` (`self.Blackboard`) (`KismetStringLibrary.Conv_StringToName` "TargetActor"))
    (:`Is Not Valid`
      (bind _outactors (`GameplayStatics.GetAllActorsWithTag` "Player"))
      (`self.UpdateTargetKey` (`|GetArrayItem` _outactors)))))

(fn `UpdateSightKey`
  (params (HasLineOfSight :type Boolean))
  (`BlackboardComponent.SetValueAsBool` (`self.Blackboard`) "HasLineOfSight" HasLineOfSight))

(fn `UpdateTargetKey`
  (params (TargetActor :type "Actor Object Reference"))
  (`BlackboardComponent.SetValueAsObject` (`self.Blackboard`) "TargetActor" TargetActor))

(fn `UserConstructionScript`)