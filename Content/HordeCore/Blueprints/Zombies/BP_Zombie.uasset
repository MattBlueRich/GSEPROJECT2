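; Zombie enemy for a horde mode that picks a random skeletal mesh on spawn and caches the player character.
; Point damage drains health; non-lethal hits switch it to run speed, which Tick feeds into FloatingPawnMovement.
; Death runs once: ragdoll, capsule collision off, points reported to BP_HordeGameMode, death event called, delayed destroy.
; Physical animation and random movement-start logic is left disconnected, with a note about a spawn crash.
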(event `self.ReceivePointDamage`
  (params (Damage :type "Float (single-precision)") (DamageType :type "DamageType Object Reference") (HitLocation :type "Vector Structure") (HitNormal :type "Vector Structure") (HitComponent :type "PrimitiveComponent Object Reference") (BoneName :type Name) (ShotFromDirection :type "Vector Structure") (InstigatedBy :type "Controller Object Reference") (DamageCauser :type "Actor Object Reference") (HitInfo :type "HitResult Structure (by ref)"))
  (set `self.CurrentHealth` (- (`self.CurrentHealth`) Damage))
  (bind _isdead (`self.Is Dead`))
  (if _isdead
    (`/Engine/EditorBlueprintResources/StandardMacros.DoOnce` false
      (:`Completed`
        (`self.Ragdoll mesh`)
        (`PrimitiveComponent.SetCollisionEnabled` (`self.Capsule`) "NoCollision")
        (bind _asbp_horde_game_mode (cast `/Game/HordeCore/Blueprints/Game/BP_HordeGameMode` (`GameplayStatics.GetGameMode`)))
        (`/Game/HordeCore/Blueprints/Game/BP_HordeGameMode.ZombieKilled` _asbp_horde_game_mode (`self.PointsReward`))
        (`self.ZombieDeath`)
        (`KismetSystemLibrary.Delay` 5.0)
        (`self.K2_DestroyActor`)))
    (else
      (set `self.Movement Speed` (`self.RunSpeed`)))))

(event `self.ReceiveBeginPlay`
  (`SkeletalMeshComponent.SetSkeletalMeshAsset` (`self.Mesh`) (`KismetArrayLibrary.Array_Random` (`self.Meshes`)))
  (bind _asbp_first_person_character (cast `/Game/FirstPerson/Blueprints/BP_FirstPersonCharacter` (`GameplayStatics.GetPlayerCharacter` 0)))
  (set `self.PlayerRef` _asbp_first_person_character)
  (`|ExecutionSequence`
    (:`then_0`
      (set `self.CurrentHealth` (`self.StartingHealth`)))))

(event `self.ReceiveTick`
  (params (DeltaSeconds :type "Float (single-precision)"))
  (set `FloatingPawnMovement.MaxSpeed` (`self.Movement Speed`) (`self.FloatingPawnMovement`)))

(fn `Is Dead`
  (returns (IsDead :type Boolean))
  (return (<= (`self.CurrentHealth`) 0.0)))

(fn `UserConstructionScript`)