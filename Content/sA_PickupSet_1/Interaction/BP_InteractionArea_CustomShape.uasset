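; BP_InteractionArea_CustomShape is an interaction area actor that takes its shape from a configurable skeletal mesh.
; On construction, SetupMeshData assigns CustomShape to the WeaponShape component, then runs the parent construction script.
; In DeveloperMode every material slot gets the M_InteractionTraceShape material to show the shape; otherwise the mesh is hidden.
; The event graph is empty, so this Blueprint adds only construction-time setup.
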(fn `Setup Mesh Data`
  (`SkeletalMeshComponent.SetSkeletalMeshAsset` (`self.WeaponShape`) (`self.CustomShape`))
  (if (`self.DeveloperMode`)
    (for _array_element (`MeshComponent.GetMaterialSlotNames` (`self.WeaponShape`))
      (`PrimitiveComponent.SetMaterialByName` (`self.WeaponShape`) _array_element "/Game/sA_PickupSet_1/Interaction/M_InteractionTraceShape.M_InteractionTraceShape"))
    (else
      (`SceneComponent.SetVisibility` (`self.WeaponShape`) false false)))
  (`parent.UserConstructionScript`))

(fn `UserConstructionScript`
  (`self.Setup Mesh Data`))