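; AC_InteractionTrace is an interaction component that detects which interaction area the player is looking at.
; Every tick it line-traces forward from the player camera on the Visibility channel and reacts when the hit actor changes.
; Hits whose class is exactly the Box or CustomShape interaction area are cast to BP_InteractionArea_Master and get ToggleFocus on.
; Other hits or misses unfocus the tracked area.
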(event `self.ReceiveTick`
  (params (DeltaSeconds :type "Float (single-precision)"))
  (`self.Trace`))

(fn `Trace`
  (bind _returnvalue (`GameplayStatics.GetPlayerCameraManager` 0))
  (bind _returnvalue_2 (`Actor.K2_GetActorLocation` _returnvalue))
  ;[1 1 1] This shoots a raycast forward, from the first-person camera. Line Trace By Channel returns either "True" or "False" if the raycast hits an object. Break Hit Result returns the object hit.
  (bind (_outhit _returnvalue_3) (`KismetSystemLibrary.LineTraceSingle` _returnvalue_2 (+ _returnvalue_2 (* (`KismetMathLibrary.GetForwardVector` (`Actor.K2_GetActorRotation` _returnvalue)) (`self.Length`))) "TraceTypeQuery1"))
  ;[1 1 1] If the object hit is new, set FocusedActor to the new object. If FocusesActor is in the BP_InteractionArea, then "Trace"!
  (if _returnvalue_3
    (bind (_bblockinghit _binitialoverlap _time _distance _location _impactpoint _normal _impactnormal _physmat _hitactor) (`GameplayStatics.BreakHitResult` _outhit))
    (if (!= (`self.FocusedActor`) _hitactor)
      (set `self.FocusedActor` _hitactor)
      (bind _returnvalue_4 (`GameplayStatics.GetObjectClass` _hitactor))
      (`self.TraceInteractionArea` (or (== _returnvalue_4 "/Game/sA_PickupSet_1/Interaction/BP_InteractionArea_Box.BP_InteractionArea_Box_C") (== _returnvalue_4 "/Game/sA_PickupSet_1/Interaction/BP_InteractionArea_CustomShape.BP_InteractionArea_CustomShape_C"))))
    (else
      (`self.TraceInteractionArea` false))))

(fn `TraceInteractionArea`
  (params (Trace :type Boolean))
  (if Trace
    (if (`self.IsTracingInteractionArea`)
      (`/Game/sA_PickupSet_1/Interaction/BP_InteractionArea_Master.ToggleFocus` (`self.FocusedInteractionArea`) false))
    (bind _asbp_interaction_area (cast `/Game/sA_PickupSet_1/Interaction/BP_InteractionArea_Master` (`self.FocusedActor`)))
    (bind _output_get (set `self.FocusedInteractionArea` _asbp_interaction_area))
    (`/Game/sA_PickupSet_1/Interaction/BP_InteractionArea_Master.ToggleFocus` _output_get true)
    (set `self.IsTracingInteractionArea` true)
    (elif (`self.IsTracingInteractionArea`)
      (set `self.IsTracingInteractionArea` false)
      (`/Game/sA_PickupSet_1/Interaction/BP_InteractionArea_Master.ToggleFocus` (`self.FocusedInteractionArea`) false)
      (set `self.FocusedActor` null)
      (set `self.FocusedInteractionArea` null))))